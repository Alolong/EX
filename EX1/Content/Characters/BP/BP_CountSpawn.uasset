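; BP_CountSpawn is a counter Blueprint that tallies overlaps on its Cube and shows the count in a widget.
; Each begin overlap increments Count without checking which actor entered.
; While Count is at most three, it prints the value and passes it to CountBox on the Widget component's WBP_CountBox.
; Later overlaps still increment Count but update nothing, and despite the name nothing is spawned here.
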(event OnComponentBeginOverlap(Cube)
  (params (OverlappedComponent :type Primitive%20Component%20Object%20Reference) (OtherActor :type Actor%20Object%20Reference) (OtherComp :type Primitive%20Component%20Object%20Reference) (OtherBodyIndex :type Integer) (bFromSweep :type Boolean) (SweepResult :type Hit%20Result%20Structure%20%28by%20ref%29))
  ;[0.15 0.15 0.15 0.5] 더해지는 식
  (bind _output_get (Variables|Default|SetCount (+ (Variables|Default|GetCount) 1)))
  (if (<= _output_get 3)
    (Development|PrintString (Utilities|String|Append "count" (Utilities|String|ToString(Integer) _output_get)))
    ;[0.15 0.15 0.15 0.5] 위젯의 기능을 가져오는 식
    (bind _aswbp_count_box (Utilities|Casting|CastToWBP_CountBox (UserInterface|GetUserWidgetObject (Variables|Default|GetWidget))))
    ;[0.15 0.15 0.15 0.5] 위젯의 카운트 박스 함수에 +식을 넣음
    (Default|CountBox _aswbp_count_box (Variables|Default|GetCount))))

(fn ConstructionScript)