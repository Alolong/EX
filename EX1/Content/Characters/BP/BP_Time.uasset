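; BP_Time is an elapsed-time clock that shows minutes and seconds on the player's HUD.
; Tick accumulates delta seconds into a running total, splits it into minutes and seconds, and sends the joined string to UpdateTime on BP_HUD every frame.
; The Floor00 helper floors each value and adds a leading zero below ten.
; A failed HUD cast just prints a debug string.
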(event EventBeginPlay)

(event EventTick
  (params (DeltaSeconds :type Float%20%28single-precision%29))
  ;[0.15 0.15 0.15 0.5] 증가식
  (bind _output_get (Variables|Default|SetTotal%20deltasecond (+ DeltaSeconds (Variables|Default|GetTotal%20deltasecond))))
  ;[0.15 0.15 0.15 0.5] 플레이어컨트롤러에서 허드를 가져와서 BP_hud로 만든다
  (bind _asbp_hud (Utilities|Casting|CastToBP_HUD (HUD|GetHUD (Game|GetPlayerController 0)))
    (:then
      (Default|UpdateTime _asbp_hud (Utilities|String|Append (CallFunction|Floor00 (/ _output_get 6e+01)) ":" (CallFunction|Floor00 (Math|Float|%(Float) _output_get 6e+01)))))
    (:CastFailed
      (Development|PrintString "Hello"))))

(fn ConstructionScript)

(fn Floor00
  (params (A :type Float%20%28double-precision%29))
  (bind _returnvalue (Math|Float|Floor A))
  (bind _returnvalue_2 (Utilities|String|ToString(Integer) _returnvalue))
  ;[0.15 0.15 0.15 0.5] 받는값이 10 이하면,
  (if (< A 1e+01)
    ;[0.15 0.15 0.15 0.5] True-앞에 0을 붙여 작성
    (return (Utilities|String|Append "0" _returnvalue_2))
    (else
      ;[0.15 0.15 0.15 0.5] false-10이상일시 계속 출력됨 10..11..12
      (return _returnvalue_2))))